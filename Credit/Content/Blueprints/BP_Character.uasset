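; Player character with forward movement, 90-degree snap turning and two single-use timed abilities: Levitation and Time Slow.
; The ability input switches on CurrentAbility, whose start function clears it, then a Delay leads to the end function.
; Levitation raises the actor in Flying mode, then restores Walking.
; Time Slow lowers global time dilation while inverse custom dilation keeps the character at normal speed.
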(event `EnhancedInput|/Game/Inputs/IA_MoveForward`
  (params (ActionValue :type "Float (double-precision)") (ElapsedSeconds :type "Float (double-precision)") (TriggeredSeconds :type "Float (double-precision)") (InputAction :type "InputAction Object Reference" :default "/Game/Inputs/IA_MoveForward.IA_MoveForward"))
  (bind (_returnvalue_roll _returnvalue_pitch _returnvalue_yaw) (`KismetMathLibrary.BreakRotator` (`self.GetControlRotation`)))
  (:`Triggered`
    (`self.AddMovementInput` (`KismetMathLibrary.GetForwardVector` (`KismetMathLibrary.MakeRotator` 0.0 0.0 _returnvalue_yaw)) ActionValue)))

(event `EnhancedInput|/Game/Inputs/IA_Look`
  (params (ActionValue :type "Float (double-precision)") (ElapsedSeconds :type "Float (double-precision)") (TriggeredSeconds :type "Float (double-precision)") (InputAction :type "InputAction Object Reference" :default "/Game/Inputs/IA_Look.IA_Look"))
  (:`Started`
    (`Controller.SetControlRotation` (`self.GetController`) (`KismetMathLibrary.ComposeRotators` (`self.GetControlRotation`) (`KismetMathLibrary.MakeRotator` 0.0 0.0 (* ActionValue (`KismetMathLibrary.Conv_IntToDouble` 90)))))))

(event `EnhancedInput|/Game/Inputs/IA_ActivateAbility`
  (params (ActionValue :type Boolean) (ElapsedSeconds :type "Float (double-precision)") (TriggeredSeconds :type "Float (double-precision)") (InputAction :type "InputAction Object Reference" :default "/Game/Inputs/IA_ActivateAbility.IA_ActivateAbility"))
  (:`Triggered`
    (switch `/Game/Blueprints/E_AbilityType` (`self.CurrentAbility `)
      (:`NewEnumerator1`
        (`self.StartLevitation`)
        (`KismetSystemLibrary.Delay` 2.0)
        (`KismetSystemLibrary.PrintString` "Stop Levitate")
        (`self.EndLevitation`))
      (:`NewEnumerator2`
        (`self.StartTimeSlow`)
        (`KismetSystemLibrary.Delay` 1.5)
        (`KismetSystemLibrary.PrintString` "Stop Time")
        (`self.EndTimeSlow`)))))

(fn `EndLevitation`
  (set `self.AbilityActive` false)
  (`CharacterMovementComponent.SetMovementMode` (`self.CharacterMovement`) "MOVE_Walking" 0))

(fn `EndTimeSlow`
  (`GameplayStatics.SetGlobalTimeDilation` 1.0)
  (set `self.CustomTimeDilation` 1.0)
  (set `self.AbilityActive` false))

(fn `StartLevitation`
  (bind (_returnvalue_x _returnvalue_y _returnvalue_z) (`KismetMathLibrary.BreakVector` (`self.K2_GetActorLocation`)))
  (bind (_returnvalue_x_2 _returnvalue_y_2 _returnvalue_z_2) (`KismetMathLibrary.BreakVector` (`self.K2_GetActorLocation`)))
  (set `self.AbilityActive` true)
  (set `self.CurrentAbility ` "NewEnumerator0")
  (set `self.OriginalHeight` _returnvalue_z)
  (`CharacterMovementComponent.SetMovementMode` (`self.CharacterMovement`) "MOVE_Flying" 0)
  (`self.K2_SetActorLocation` (`KismetMathLibrary.MakeVector` _returnvalue_x_2 _returnvalue_y_2 (+ _returnvalue_z_2 (`self.LevitationHeight`)))))

(fn `StartTimeSlow`
  (set `self.AbilityActive` true)
  (set `self.CurrentAbility ` "NewEnumerator0")
  (`GameplayStatics.SetGlobalTimeDilation` 0.3)
  (set `self.CustomTimeDilation` 3.33))

(fn `UserConstructionScript`)